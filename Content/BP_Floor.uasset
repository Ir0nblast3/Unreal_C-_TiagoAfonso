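; BP_Floor is a floor tile that extends the level as the player advances and can hold obstacles in three lanes.
; When the player character overlaps DestroyBox, it asks BP_ThirdPersonGameMode to add a floor, then destroys itself.
; SpawnObstacle picks one of three spawn points by lane number and adds the given class there as a child actor component.
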(event `self.Destroy Box.OnComponentBeginOverlap`
  (params (OverlappedComponent :type "PrimitiveComponent Object Reference") (OtherActor :type "Actor Object Reference") (OtherComp :type "PrimitiveComponent Object Reference") (OtherBodyIndex :type Integer) (bFromSweep :type Boolean) (SweepResult :type "HitResult Structure (by ref)"))
  (if (== OtherActor (`GameplayStatics.GetPlayerCharacter` 0))
    (bind _asbp_third_person_game_mode (cast `/Game/ThirdPerson/Blueprints/BP_ThirdPersonGameMode` (`GameplayStatics.GetGameMode`)))
    (`/Game/ThirdPerson/Blueprints/BP_ThirdPersonGameMode.Add Floor` _asbp_third_person_game_mode)
    (`self.K2_DestroyActor`)))

(event `Spawn Obstacle`
  (params (`Obstacle Class` :type "/Game/Objects/BP_Obstacles Class Reference") (`Lane No` :type Integer))
  (bind _returnvalue (`AddComponent|NODE_AddChildActorComponent-0` :`RelativeTransform` (`KismetMathLibrary.MakeTransform` (`SceneComponent.RelativeLocation` (select `int` `Lane No` :`0` (`self.SpawnPoint1`) :`1` (`self.SpawnPoint2`) :`2` (`self.SpawnPoint3`))))))
  (`ChildActorComponent.SetChildActorClass` _returnvalue `Obstacle Class`))

(fn `UserConstructionScript`)